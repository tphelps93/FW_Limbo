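; BP_PlayerCtrl is the player controller for John, which sets up the player's UI and caches core references at BeginPlay.
; It stores the game instance, game state and player character, with each failed cast halting the rest of setup.
; It then creates pickup message, crosshair, pause and tab menu widgets and adds them all to the viewport.
; Inventory and journal references come from child widgets of the tab menu.
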(event EventBeginPlay
  ;[0.05098 0.05098 0.05098] Get Game Instance
  (bind _asmy_game_instance (Utilities|Casting|CastToMyGameInstance (Game|GetGameInstance)))
  (Variables|Default|SetMyGameInstance _asmy_game_instance)
  ;[0.05098 0.05098 0.05098] Get Game State
  (bind _asbp_game_state (Utilities|Casting|CastToBP_GameState (Game|GetGameState)))
  (Utilities|IsValid _asbp_game_state
    (:Is%20Valid
      (Variables|Default|SetGameState _asbp_game_state)
      ;[0.05098 0.05098 0.05098] Get Player John
      (bind _asbp_player_john (Utilities|Casting|CastToBP_Player_John (Game|GetPlayerCharacter 0)))
      (Variables|Default|SetPlayerJohn _asbp_player_john)
      ;[0.05098 0.05098 0.05098] Get Pickup Message Widget
      (bind _returnvalue (UserInterface|CreateWidget "/Game/_Characters/Player_John/UI_Elements/UI_PickUpMessage.UI_PickUpMessage_C" (Game|GetPlayerController 0)))
      (Utilities|IsValid _returnvalue
        (:Is%20Valid
          (bind _output_get (Variables|Default|SetInteractionMessageWidget _returnvalue))
          (UserInterface|Viewport|AddtoViewport _output_get 0)
          ;[0.05098 0.05098 0.05098] Get CrossHair Widget
          (bind _returnvalue_2 (UserInterface|CreateWidget "/Game/_Characters/Player_John/UI_Elements/UI_CrossHair.UI_CrossHair_C" (Game|GetPlayerController 0)))
          (bind _output_get_2 (Variables|Default|SetCrosshair _returnvalue_2))
          (UserInterface|Viewport|AddtoViewport _output_get_2 0)
          ;[0.05098 0.05098 0.05098] Get Pause Menu Widget
          (bind _returnvalue_3 (UserInterface|CreateWidget "/Game/_Characters/Player_John/UI_Elements/UI_PauseMenu.UI_PauseMenu_C" (Game|GetPlayerController 0)))
          (bind _output_get_3 (Variables|Default|SetPauseMenuWidget _returnvalue_3))
          (UserInterface|Viewport|AddtoViewport _output_get_3 0)
          ;[0.05098 0.05098 0.05098] Get Tab Menu Widget
          (bind _returnvalue_4 (UserInterface|CreateWidget "/Game/_Characters/Player_John/UI_Elements/TabMenu/UI_TabMenu.UI_TabMenu_C" (Game|GetPlayerController 0)))
          (bind _output_get_4 (Variables|Default|SetTabMenuWidget _returnvalue_4))
          (UserInterface|Viewport|AddtoViewport _output_get_4 0)
          ;[0.05098 0.05098 0.05098] Get Inventory Widget
          (Variables|Default|SetInventoryWidget (Variables|/Game/_Characters/Player_John/UI_Elements/TabMenu/UI_TabMenu.UI_TabMenu_C|GetUI_Inventory _returnvalue_4))
          ;[0.05098 0.05098 0.05098] Get Journal Widget
          (Variables|Default|SetJournalWidget (Variables|/Game/_Characters/Player_John/UI_Elements/TabMenu/UI_TabMenu.UI_TabMenu_C|GetUI_JournalMenu _returnvalue_4)))))))

(fn ConstructionScript)