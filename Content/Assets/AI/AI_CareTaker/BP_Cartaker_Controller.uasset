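; AI controller for the CareTaker that runs its behavior tree and reacts to perception.
; Sight updates store the actor as TargetActor on the blackboard and set Panic on the game state, without checking tag or sensing success.
; Other senses store the stimulus location as TargetLocation.
; Player-tag line-of-sight logic with a lose-sight timer is present but disconnected.
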(event OnTargetPerceptionUpdated(AIPerception)
  (params (Actor :type Actor%20Object%20Reference) (Stimulus :type AI%20Stimulus%20Structure))
  (bind _returnvalue (Class|AIPerceptionSystem|GetSenseClassforStimulus Stimulus))
  (if (== _returnvalue "/Script/AIModule.AISense_Sight")
    (AI|Components|Blackboard|SetValueasObject (Variables|Default|GetBlackboard) (Utilities|Name|MakeLiteralName "TargetActor") Actor)
    (Variables|/Game/Assets/Sun_Moon_Cycle/BP_GameState.BP_GameState_C|SetPanic (Variables|Default|GetGameState) true)
    (else
      (AI|Components|Blackboard|SetValueasVector (Variables|Default|GetBlackboard) (Utilities|Name|MakeLiteralName "TargetLocation") (.StimulusLocation (Utilities|Struct|BreakAIStimulus Stimulus))))))

(event Custom|StartEnemyTimer
  (bind _blackboard (Variables|Default|GetBlackboard))
  (AI|Components|Blackboard|SetValueasBool _blackboard (Variables|Default|GetHasLineOfSight) false)
  (AI|Components|Blackboard|SetValueasObject _blackboard (Variables|Default|GetCaretaker) 0))

(event EventBeginPlay
  (AI|RunBehaviorTree "/Game/Assets/AI/AI_CareTaker/BT_CareTaker.BT_CareTaker")
  (bind _asbp_game_state (Utilities|Casting|CastToBP_GameState (Game|GetGameState)))
  (Variables|Default|SetGameState _asbp_game_state))

(fn ConstructionScript)