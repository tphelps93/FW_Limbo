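; Interactable locker that the player can enter to hide and exit again, with prompt text that follows the GameState's PlayerIsHiding flag.
; The hit normal against the door collision's forward vector tells entering from leaving.
; Timelines swing the door and lerp the player in or out, sequenced by delays with sound, camera shake and a 180-degree turn.
; Entering unequips the flashlight and narrows view limits, leaving widens them, and closing updates the hiding flag.
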(event Custom|LockerDoorOpen
  (bind (_world_location _world_rotation) (Utilities|GetLockerDoorLocation))
  ;[0.05098 0.05098 0.05098] Locker Door Opening and Closing
  (Audio|PlaySoundatLocation "/Game/Assets/SFX/LockerOpen/Locker_Open_Cue.Locker_Open_Cue" _world_location _world_rotation 1.0 1.0 0.0 "/Game/Assets/SFX/DoorOpening/DoorAtten.DoorAtten" 0 0 0)
  (bind _locker_door_track (Timeline|T_LockerDoorOpen Play)
    (:Update
      (Transformation|SetRelativeRotation (Variables|Default|GetLocker_Door) (Math|Rotator|MakeRotator 0.0 0.0 (Utilities|LockerDoorLerp _locker_door_track)) false false))
    (:Finished
      (Variables|DoorStates|SetisOpen? (not (Variables|DoorStates|GetisOpen?))))))

(event Custom|LockerDoorClose
  ;[0.05098 0.05098 0.05098] Locker Door Opening and Closing
  (bind _locker_door_track (Timeline|T_LockerDoorOpen Reverse)
    (:Update
      (Transformation|SetRelativeRotation (Variables|Default|GetLocker_Door) (Math|Rotator|MakeRotator 0.0 0.0 (Utilities|LockerDoorLerp _locker_door_track)) false false))
    (:Finished
      (Variables|DoorStates|SetisOpen? (not (Variables|DoorStates|GetisOpen?))))))

(event Custom|MovePlayerIn/OutOfLocker
  ;[0.05098 0.05098 0.05098] Move Player in and out of Locker
  (bind _moveto (Timeline|T_MovePlayerIn/OutOfLocker PlayFromStart)
    (:Update
      (Transformation|SetActorLocation (Game|GetPlayerCharacter 0) (Utilities|LerpIn/OutOfLocker _moveto) false false))
    (:Finished
      (Variables|DoorStates|SetisAnimPlaying? false))))

(event EventBeginPlay
  ;[0.05098 0.05098 0.05098] Cast player character and set to variable on BeginPlay
  ;;[1 1 1] Get Player Character
  (bind _asbp_player_john (Utilities|Casting|CastToBP_Player_John (Game|GetPlayerCharacter 0)))
  (Variables|BPReferences|SetPlayer%20John _asbp_player_john)
  ;;[1 1 1] Get Game State
  (bind _asbp_game_state (Utilities|Casting|CastToBP_GameState (Game|GetGameState)))
  (Variables|BPReferences|SetGameState _asbp_game_state)
  ;;[1 1 1] Get Interaction Message Widget
  (bind _returnvalue (UserInterface|CreateWidget "/Game/_Characters/Player_John/UI_Elements/UI_PickUpMessage.UI_PickUpMessage_C"))
  (bind _output_get (Variables|Interaction|SetInteractionMessageWidget _returnvalue))
  (UserInterface|Viewport|AddtoViewport _output_get 0))

(event EventInteract
  (params (Out%20Hit%20Normal :type Vector :default "0, 0, 0"))
  ;[0.05098 0.05098 0.05098] Interact with Locker Door
  (if (not (Variables|DoorStates|GetisAnimPlaying?))
    (if (not (Variables|DoorStates|GetisOpen?))
      (Utilities|GetFrontOfDoor Out%20Hit%20Normal
        (:then
          _)
        (:Else
          (Utilities|GetBackOfDoor Out%20Hit%20Normal)))
      (Variables|DoorStates|SetisAnimPlaying? true)
      (Utilities|OpenLockerDoor)
      (else
        (Variables|DoorStates|SetisAnimPlaying? true)
        (Utilities|CloseLockerDoor)))))

(fn ConstructionScript)

(fn RotatePlayer180Degrees
  (bind (_player_controller _rotation) (Utilities|RotatePlayer-180))
  (bind (_playercontroller _rotation_2) (Utilities|RotatePlayer180))
  (Utilities|ControllerRotationLagToggle)
  (if (Variables|DoorStates|GetisFrontOfDoor)
    (Pawn|SetControlRotation _playercontroller _rotation_2)
    (elif (Variables|DoorStates|GetisBackOfDoor)
      (Pawn|SetControlRotation _player_controller _rotation))))

(fn IsSelected?
  (return false))

(fn Lookat
  (params (Observer :type BP%20Player%20John%20Object%20Reference))
  (if (Variables|/Game/Assets/Sun_Moon_Cycle/BP_GameState.BP_GameState_C|GetplayerIsHiding? (Variables|BPReferences|GetGameState))
    (return (Variables|Interaction|GetInteractionText_Hiding))
    (else
      (return (Variables|Interaction|GetInteractionText_NotHiding)))))