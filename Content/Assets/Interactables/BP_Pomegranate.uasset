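; BP_Pomegranate is an interactable pomegranate prop that can be highlighted and looked at.
; Select and deselect events toggle custom depth rendering on its static mesh.
; LookAt returns its InteractionText regardless of the observer.
; It has no pickup or use logic, and its BeginPlay, overlap, Tick and construction script add no behavior.
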(event EventBeginPlay
  (|CallParentFunction) ; This node is disabled and will not be called.\nDrag off pins to build functionality.
)

(event Collision|EventActorBeginOverlap
  (params (OtherActor :type Actor%20Object%20Reference))
  (|CallParentFunction OtherActor) ; This node is disabled and will not be called.\nDrag off pins to build functionality.
)

(event EventTick
  (params (DeltaSeconds :type Float%20%28single-precision%29))
  (|CallParentFunction DeltaSeconds) ; This node is disabled and will not be called.\nDrag off pins to build functionality.
)

(event EventSelectInteractable
  (Rendering|SetRenderCustomDepth (Variables|Default|GetStaticMesh) true))

(event EventDeselectInteractable
  (Rendering|SetRenderCustomDepth (Variables|Default|GetStaticMesh) false))

(fn ConstructionScript
  (|CallParentFunction))

(fn Lookat
  (params (Observer :type BP%20Player%20John%20Object%20Reference))
  (return (Variables|Default|GetInteraction%20Text)))