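; Interactable old door that the player opens and closes, or that jiggles its knob when locked.
; Timelines rotate knob and door with sound cues and delays, using front or back lerps chosen from the interaction hit normal outside Panic.
; The GameState Panic flag switches to panic timings and opening sound, and closes an open door when the player leaves its bounds.
; The player move-to call for the opening animation is disconnected.
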(event OnComponentEndOverlap(PlayerBounds)
  (params (OverlappedComponent :type Primitive%20Component%20Object%20Reference) (OtherActor :type Actor%20Object%20Reference) (OtherComp :type Primitive%20Component%20Object%20Reference) (OtherBodyIndex :type Integer))
  ;[0.05098 0.05098 0.05098] Close Door when Player exits the bounds
  (if (Variables|/Game/Assets/Sun_Moon_Cycle/BP_GameState.BP_GameState_C|GetPanic (Variables|BPReferences|GetGameState))
    (Panic|PanicDoorSpeed)
    (Utilities|Casting|CastToBP_Player_John OtherActor)
    (if (not (Variables|DoorStates|GetisAnimPlaying?))
      (if (not (not (Variables|DoorStates|GetIsOpen?)))
        (Variables|DoorStates|SetisAnimPlaying? true)
        (Utilities|CloseDoor)))))

(event Custom|DoorOpen
  (bind (_worldlocation _worldrotation) (Utilities|GetDoorLocation))
  (bind _door (Variables|Default|GetDoor))
  ;[0.05098 0.05098 0.05098] Door Opening and Closing
  (Audio|PlaySoundatLocation (Variables|BPReferences|GetDoorOpenSound) _worldlocation _worldrotation 1.0 1.0 0.0 "/Game/Assets/SFX/DoorOpening/DoorAtten.DoorAtten" 0 0 0)
  (bind _doortrack (Timeline|T_DoorOpenOrClose Play)
    (:Update
      (if (Variables|DoorStates|GetisFrontOfDoor)
        (Transformation|SetRelativeRotation _door (Math|Rotator|MakeRotator 0.0 0.0 (Utilities|DoorLerpFront _doortrack)) false false)
        (CallFunction|KnobTurnClose :!label _label)
        (elif (Variables|DoorStates|GetisBackOfDoor)
          (Transformation|SetRelativeRotation _door (Math|Rotator|MakeRotator 0.0 0.0 (Utilities|DoorLerpBack _doortrack)) false false)
          (goto _label))))
    (:Finished
      (Variables|DoorStates|SetIsOpen? (not (Variables|DoorStates|GetIsOpen?)))
      (Variables|DoorStates|SetisAnimPlaying? false))))

(event Custom|DoorClose
  (bind _door (Variables|Default|GetDoor))
  ;[0.05098 0.05098 0.05098] Door Opening and Closing
  (bind _doortrack (Timeline|T_DoorOpenOrClose Reverse)
    (:Update
      (if (Variables|DoorStates|GetisFrontOfDoor)
        (Transformation|SetRelativeRotation _door (Math|Rotator|MakeRotator 0.0 0.0 (Utilities|DoorLerpFront _doortrack)) false false)
        (CallFunction|KnobTurnClose :!label _label)
        (elif (Variables|DoorStates|GetisBackOfDoor)
          (Transformation|SetRelativeRotation _door (Math|Rotator|MakeRotator 0.0 0.0 (Utilities|DoorLerpBack _doortrack)) false false)
          (goto _label))))
    (:Finished
      (Variables|DoorStates|SetIsOpen? (not (Variables|DoorStates|GetIsOpen?)))
      (Variables|DoorStates|SetisAnimPlaying? false))))

(event Custom|KnobTurnOpen
  (bind (_worldlocation _worldrotation) (Utilities|GetDoorLocation))
  (bind _door_knob_01 (Variables|Default|GetDoor_Knob_01))
  ;[0.05098 0.05098 0.05098] Door Knob Turning
  (Audio|PlaySoundatLocation "/Game/Assets/SFX/DoorKnob/DoorKnob_Turn_Cue.DoorKnob_Turn_Cue" _worldlocation _worldrotation 1.0 1.0 0.0 "/Game/Assets/SFX/DoorOpening/DoorAtten.DoorAtten" 0 0 0)
  (bind _doorknobturn (Timeline|T_DoorKnobTurn Play)
    (:Update
      (if (Variables|DoorStates|GetisFrontOfDoor)
        (Transformation|SetRelativeRotation _door_knob_01 (Math|Rotator|MakeRotator 0.0 (Utilities|DoorKnobLerpFront _doorknobturn) 0.0) false false)
        (elif (Variables|DoorStates|GetisBackOfDoor)
          (Transformation|SetRelativeRotation _door_knob_01 (Math|Rotator|MakeRotator 0.0 (Utilities|DoorKnobLerpBack _doorknobturn) 0.0) false false))))))

(event Custom|KnobTurnClose
  (bind _door_knob_01 (Variables|Default|GetDoor_Knob_01))
  ;[0.05098 0.05098 0.05098] Door Knob Turning
  (bind _doorknobturn (Timeline|T_DoorKnobTurn Reverse)
    (:Update
      (if (Variables|DoorStates|GetisFrontOfDoor)
        (Transformation|SetRelativeRotation _door_knob_01 (Math|Rotator|MakeRotator 0.0 (Utilities|DoorKnobLerpFront _doorknobturn) 0.0) false false)
        (elif (Variables|DoorStates|GetisBackOfDoor)
          (Transformation|SetRelativeRotation _door_knob_01 (Math|Rotator|MakeRotator 0.0 (Utilities|DoorKnobLerpBack _doorknobturn) 0.0) false false))))))

(event Custom|DoorLocked
  (bind (_worldlocation _worldrotation) (Utilities|GetDoorLocation))
  ;[0.05098 0.05098 0.05098] Door Knob Locked
  (Audio|PlaySoundatLocation "/Game/Assets/SFX/DoorLocked/Door_Knob_Jiggle_Cue.Door_Knob_Jiggle_Cue" _worldlocation _worldrotation 1.0 1.0 0.0 "/Game/Assets/SFX/DoorOpening/DoorAtten.DoorAtten" 0 0 0)
  (bind _doorknoblocked (Timeline|T_DoorKnobLocked PlayFromStart)
    (:Update
      (Transformation|SetRelativeRotation (Variables|Default|GetDoor_Knob_01) (Math|Rotator|MakeRotator 0.0 (Utilities|DoorKnobLerpFront _doorknoblocked) 0.0) false false))))

(event EventBeginPlay
  ;[0.05098 0.05098 0.05098] Cast player character and set to variable on BeginPlay
  (bind _asbp_player_john (Utilities|Casting|CastToBP_Player_John (Game|GetPlayerCharacter 0)))
  (Variables|BPReferences|SetPlayerJohn _asbp_player_john)
  (bind _asbp_game_state (Utilities|Casting|CastToBP_GameState (Game|GetGameState)))
  (Variables|BPReferences|SetGameState _asbp_game_state)
  (bind _returnvalue (UserInterface|CreateWidget "/Game/_Characters/Player_John/UI_Elements/UI_PickUpMessage.UI_PickUpMessage_C"))
  (UserInterface|Viewport|AddtoViewport _returnvalue 0))

(event EventInteract
  (params (Out%20Hit%20Normal :type Vector :default "0, 0, 0"))
  ;[0.05098 0.05098 0.05098] Interact with Door
  (if (Variables|DoorStates|GetisDoorLocked?)
    (if (not (Variables|DoorStates|GetisAnimPlaying?))
      (if (not (Variables|DoorStates|GetIsOpen?))
        (CallFunction|DoorLocked)))
    (else
      ;;[0.09412 0.4275 0 1 10] Sets door anim speeds based on if the player is being chased or not
      (Panic|PanicDoorSpeed)
      (if (not (Variables|DoorStates|GetisAnimPlaying?))
        (if (not (Variables|DoorStates|GetIsOpen?))
          ;;[0.09412 0.4275 0 1 10] Sets the point for the player to move to when opening the door for the animation to the FRONT of the door
          (Utilities|SetMovetoPointtoFront Out%20Hit%20Normal
            (:then
              _)
            (:else
              ;;[0.09412 0.4275 0 1 10] Sets the point for the player to move to when opening the door for the animation to the BACK of the door
              (Utilities|SetMovetoPointtoBack Out%20Hit%20Normal)))
          (Variables|DoorStates|SetisAnimPlaying? true)
          (Utilities|OpenDoor)
          (else
            (Variables|DoorStates|SetisAnimPlaying? true)
            (Utilities|CloseDoor)))))))

(fn ConstructionScript)

(fn PanicDoorSpeed
  (bind _t_doorknobturn (Variables|Default|GetT_DoorKnobTurn))
  (if (Variables|/Game/Assets/Sun_Moon_Cycle/BP_GameState.BP_GameState_C|GetPanic (Variables|BPReferences|GetGameState))
    (Variables|BPReferences|SetDoorOpenSound "/Game/Assets/SFX/DoorOpening/Door_Opening_Fast_Cue.Door_Opening_Fast_Cue")
    (Variables|Timing|SetTimeToOpen%28s%29 (Variables|Panic|GetPanic%20Time%20to%20Open%28s%29))
    (Variables|Timing|SetTimeToClose%28s%29 (Variables|Panic|GetPanic%20Time%20to%20Close%28s%29))
    (Components|Timeline|SetPlayRate _t_doorknobturn (/ 1.0 (Variables|Panic|GetPanic%20Time%20to%20Turn%28s%29)))
    (Variables|Timing|SetCloseDoorSoundDelay 0.7)
    (Variables|Timing|SetKnobTurnToOpenDelay 0.2)
    (else
      (Variables|BPReferences|SetDoorOpenSound "/Game/Assets/SFX/DoorOpening/Door_Opening_Cue.Door_Opening_Cue")
      (Variables|Timing|SetTimeToOpen%28s%29 (Variables|Calm|GetCalm%20Time%20to%20Open%28s%29))
      (Variables|Timing|SetTimeToClose%28s%29 (Variables|Calm|GetCalm%20Time%20to%20Close%28s%29))
      (Components|Timeline|SetPlayRate _t_doorknobturn (/ 1.0 (Variables|Calm|GetCalm%20Time%20to%20Turn%28s%29)))
      (Variables|Timing|SetCloseDoorSoundDelay 1.8)
      (Variables|Timing|SetKnobTurnToOpenDelay 0.8))))

(fn IsSelected?
  (return false))

(fn Lookat
  (params (Observer :type BP%20Player%20John%20Object%20Reference))
  (if (Variables|DoorStates|GetIsOpen?)
    (return (Variables|Interaction|GetInteractionText_Open))
    (else
      (return (Variables|Interaction|GetInteractionText_Closed)))))