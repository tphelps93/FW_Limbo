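; BP_Journal is an interactable journal actor that the player can read and put down.
; Selection toggles custom depth on its mesh, and LookAt returns a read or put-down prompt based on the game state's IsJournalOpen flag.
; Interact flips that flag, adding or removing a UI_Journal widget filled with JournalContent while switching input mode and blocking or restoring movement.
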(event EventBeginPlay
  ;[0.05098 0.05098 0.05098] On BeginPlay - Get Assets
  ;;[1 1 1] Get Journal Widget
  (bind _returnvalue (UserInterface|CreateWidget "/Game/Assets/Interactables/Journal/UI_Journal.UI_Journal_C"))
  (Variables|BPReferences|SetJournalWidget _returnvalue)
  ;;[1 1 1] Get Game State
  (bind _asbp_game_state (Utilities|Casting|CastToBP_GameState (Game|GetGameState)))
  (Variables|BPReferences|SetGameState _asbp_game_state)
  ;;[1 1 1] Get Interaction Message Widget
  (bind _returnvalue_2 (UserInterface|CreateWidget "/Game/_Characters/Player_John/UI_Elements/UI_PickUpMessage.UI_PickUpMessage_C"))
  (Variables|Interaction|SetInteractionMessageWidget _returnvalue_2))

(event Collision|EventActorBeginOverlap
  (params (OtherActor :type Actor%20Object%20Reference)))

(event EventTick
  (params (DeltaSeconds :type Float%20%28single-precision%29)))

(event EventInteract
  (params (Out%20Hit%20Normal :type Vector :default "0, 0, 0"))
  (bind _returnvalue (Game|GetPlayerController 0))
  (if (Variables|/Game/Assets/Sun_Moon_Cycle/BP_GameState.BP_GameState_C|GetisJournalOpen? (Variables|BPReferences|GetGameState))
    (Input|SetIgnoreMoveInput _returnvalue false)
    (Input|SetInputModeGameOnly _returnvalue false)
    (Variables|/Game/Assets/Sun_Moon_Cycle/BP_GameState.BP_GameState_C|SetisJournalOpen? (Variables|BPReferences|GetGameState) false)
    (Widget|RemovefromParent (Variables|BPReferences|GetJournalWidget))
    (else
      (Input|SetIgnoreMoveInput _returnvalue true)
      (Input|SetInputModeGameandUI _returnvalue (Variables|BPReferences|GetJournalWidget) "DoNotLock" false false)
      (Variables|/Game/Assets/Sun_Moon_Cycle/BP_GameState.BP_GameState_C|SetisJournalOpen? (Variables|BPReferences|GetGameState) true)
      (UserInterface|Viewport|AddtoViewport (Variables|BPReferences|GetJournalWidget) 0)
      (Variables|/Game/Assets/Interactables/Journal/UI_Journal.UI_Journal_C|SetContentText (Variables|BPReferences|GetJournalWidget) (Variables|Default|GetJournalContent)))))

(event EventSelectInteractable
  (Rendering|SetRenderCustomDepth (Variables|Default|GetStaticMesh) true))

(event EventDeselectInteractable
  (Rendering|SetRenderCustomDepth (Variables|Default|GetStaticMesh) false))

(fn ConstructionScript)

(fn IsSelected?
  (return false))

(fn Lookat
  (params (Observer :type BP%20Player%20John%20Object%20Reference))
  (if (Variables|/Game/Assets/Sun_Moon_Cycle/BP_GameState.BP_GameState_C|GetisJournalOpen? (Variables|BPReferences|GetGameState))
    (return (Variables|Interaction|GetPutDown_InteractionText))
    (else
      (return (Variables|Interaction|GetRead_InteractionText)))))