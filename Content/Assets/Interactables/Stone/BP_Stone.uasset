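; BP_Stone is an interactable stone that the player can pick up, with an impact sound when it hits something.
; Interact calls PickupStone, which snaps it to the player's right-hand item socket, with a flashlight unequip gated by PlayerHasFlashlight, whose body is unwired.
; LookAt adds a new pickup-message widget and returns the interaction text.
; Mesh hits play an attenuated drop sound, throttled by a DoOnce with a delayed reset.
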(event OnComponentHit(StaticMesh)
  (params (HitComponent :type Primitive%20Component%20Object%20Reference) (OtherActor :type Actor%20Object%20Reference) (OtherComp :type Primitive%20Component%20Object%20Reference) (NormalImpulse :type Vector :default "0, 0, 0") (Hit :type Hit%20Result%20Structure%20%28by%20ref%29))
  (bind _staticmesh (Variables|Default|GetStaticMesh))
  (Utilities|FlowControl|DoOnce false :!label _label
    (:Completed
      (Audio|PlaySoundatLocation "/Game/Assets/SFX/Stone/stone-drop.stone-drop" (Transformation|GetWorldLocation _staticmesh) (Transformation|GetWorldRotation _staticmesh) 0.4 1.0 0.0 "/Game/Assets/SFX/Stone/Atten_StoneDrop.Atten_StoneDrop" 0 0 0)
      (Utilities|FlowControl|Delay 1.0)
      (goto _label Reset))))

(event EventBeginPlay
  (|CallParentFunction)
  (bind _asbp_player_john (Utilities|Casting|CastToBP_Player_John (Game|GetPlayerCharacter 0)))
  (Variables|Default|SetPlayerJohn _asbp_player_john)
  (Utilities|FlowControl|Delay 5.0))

(event Collision|EventActorBeginOverlap
  (params (OtherActor :type Actor%20Object%20Reference))
  (|CallParentFunction OtherActor))

(event EventTick
  (params (DeltaSeconds :type Float%20%28single-precision%29))
  (|CallParentFunction DeltaSeconds) ; This node is disabled and will not be called.\nDrag off pins to build functionality.
)

(event EventInteract
  (params (Out%20Hit%20Normal :type Vector :default "0, 0, 0"))
  (CallFunction|PickupStone))

(fn ConstructionScript
  (|CallParentFunction))

(fn PickupStone
  (if (not (Variables|Default|GetisHoldingStone?))
    (if (Utilities|PlayerHasFlashlight)
      (Default|UnequipFlashlight (Variables|Default|GetPlayerJohn)))
    (Transformation|AttachComponentToComponent (Variables|/Game/_Characters/Player_John/BP_Player_John.BP_Player_John_C|GetUseItem (Variables|Default|GetPlayerJohn)) "item_r_SOCKET" "SnapToTarget" "SnapToTarget" "SnapToTarget" true)
    (Variables|Default|SetisHoldingStone? true)))

(fn Lookat
  (params (Observer :type BP%20Player%20John%20Object%20Reference))
  (bind _returnvalue (UserInterface|CreateWidget "/Game/_Characters/Player_John/UI_Elements/UI_PickUpMessage.UI_PickUpMessage_C"))
  (UserInterface|Viewport|AddtoViewport _returnvalue 0)
  (return (Variables|Default|GetInteractionText)))