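; Game state Blueprint for a sun and moon cycle, built to advance time of day on BP_CustomSunSky.
; TimeUpdate adds seconds to a wrapping day counter, writes hours, minutes and seconds to the sky, then calls StarsOn or StarsOff by hour range.
; BeginPlay is empty: the initialization that reads the sky's start time and the looping timer driving TimeUpdate are disconnected, so the file never starts the clock.
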(event Custom|TimeUpdate
  (Utilities|FlowControl|Sequence
    (:then_0
      (CallFunction|AdvanceTime))
    (:then_1
      (|StarsOn/Off[EVENTS]))))

(event EventBeginPlay)

(fn ConstructionScript)

(fn AdvanceTime
  (bind _sunsky (Variables|Default|GetSunSky))
  (bind _output_get (Variables|Default|SetTimeOfDayInSeconds (+ (Variables|Default|GetTimeOfDayInSeconds) (Variables|Default|GetSecondsToAddPerTick))))
  (Variables|/Game/Assets/Sun_Moon_Cycle/BP_CustomSunSky.BP_CustomSunSky_C|SetHours _sunsky (.Hours (Math|Timespan|BreakTimespan (Math|Timespan|MakeTimespan 0 0 0 _output_get))))
  (Variables|/Game/Assets/Sun_Moon_Cycle/BP_CustomSunSky.BP_CustomSunSky_C|SetMinutes _sunsky (.Minutes (Math|Timespan|BreakTimespan (Math|Timespan|MakeTimespan 0 0 0 _output_get))))
  (Variables|/Game/Assets/Sun_Moon_Cycle/BP_CustomSunSky.BP_CustomSunSky_C|SetSeconds _sunsky (.Seconds (Math|Timespan|BreakTimespan (Math|Timespan|MakeTimespan 0 0 0 _output_get))))
  (if (>= (Variables|Default|GetTimeOfDayInSeconds) 86400)
    (Variables|Default|SetTimeOfDayInSeconds 0)))

(fn IsCertainTime
  (params (Hours :type Integer) (Minutes :type Integer) (Seconds :type Integer))
  (return (== (Math|Timespan|MakeTimespan 0 Hours Minutes Seconds) (Math|Timespan|MakeTimespan 0 0 0 (Variables|Default|GetTimeOfDayInSeconds)))))

(fn IsOverCertainTime
  (params (Hours :type Integer) (Minutes :type Integer) (Seconds :type Integer))
  (return (> (Math|Timespan|MakeTimespan 0 Hours Minutes Seconds) (Math|Timespan|MakeTimespan 0 0 0 (Variables|Default|GetTimeOfDayInSeconds)))))

(fn IsUnderCertainTime
  (params (Hours :type Integer) (Minutes :type Integer) (Seconds :type Integer))
  (return (< (Math|Timespan|MakeTimespan 0 Hours Minutes Seconds) (Math|Timespan|MakeTimespan 0 0 0 (Variables|Default|GetTimeOfDayInSeconds)))))